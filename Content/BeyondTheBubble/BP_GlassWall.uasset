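; BP_GlassWall is a destructible glass wall actor that shatters when it takes any damage.
; On damage it spawns a Niagara shatter effect at the Glass component's transform, removes that component and plays a sound at the actor's location.
; The actor destroys itself once the particle system reports it has finished.
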(event Custom|CustomEvent
  (params (PSystem :type Niagara%20Component%20Object%20Reference))
  (Actor|DestroyActor))

(event Game|Damage|EventAnyDamage
  (params (Damage :type Float%20%28single-precision%29) (DamageType :type Damage%20Type%20Object%20Reference) (InstigatedBy :type Controller%20Object%20Reference) (DamageCauser :type Actor%20Object%20Reference))
  (bind _glass (Variables|Default|GetGlass))
  (bind _returnvalue (Niagara|SpawnSystematLocation "/Game/BeyondTheBubble/Material/NS_Destructable_glass.NS_Destructable_glass" (Transformation|GetWorldLocation _glass) (Transformation|GetWorldRotation _glass) (Transformation|GetWorldScale _glass)))
  (Components|DestroyComponent (Variables|Default|GetGlass))
  (EventDispatchers|BindEventtoOnSystemFinished _returnvalue (delegate Custom|CustomEvent))
  (Audio|PlaySoundatLocation "/Engine/VREditor/Sounds/UI/Foliage_Placed.Foliage_Placed" (Transformation|GetActorLocation) "0, 0, 0" 1.0 1.0 0.0 0 0 0 0))

(fn ConstructionScript)