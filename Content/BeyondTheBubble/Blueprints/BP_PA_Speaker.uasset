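; BP_PA_Speaker is a PA speaker that plays a chime and voice announcement when the first-person character enters its TriggerSphere.
; An IsActivated flag blocks retriggering and is set before the character cast, so any overlapping actor sets it.
; The voice follows the chime after a short delay.
; If the character leaves while the voice plays, it fades out and stops, then the flag resets; otherwise the flag stays set.
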(event OnComponentBeginOverlap(TriggerSphere)
  (params (OverlappedComponent :type Primitive%20Component%20Object%20Reference) (OtherActor :type Actor%20Object%20Reference) (OtherComp :type Primitive%20Component%20Object%20Reference) (OtherBodyIndex :type Integer) (bFromSweep :type Boolean) (SweepResult :type Hit%20Result%20Structure%20%28by%20ref%29))
  (if (not (Variables|Default|GetIsActivated))
    (Variables|Default|SetIsActivated true)
    (Utilities|Casting|CastToBP_FirstPersonCharacter OtherActor)
    (Audio|Components|Audio|Play (Variables|Default|GetChimeSound) 0.0)
    (Utilities|FlowControl|Delay 2.0)
    (Audio|Components|Audio|Play (Variables|Default|GetSpeakerVoice) 0.0)))

(event OnComponentEndOverlap(TriggerSphere)
  (params (OverlappedComponent :type Primitive%20Component%20Object%20Reference) (OtherActor :type Actor%20Object%20Reference) (OtherComp :type Primitive%20Component%20Object%20Reference) (OtherBodyIndex :type Integer))
  (if (Audio|Components|Audio|IsPlaying (Variables|Default|GetSpeakerVoice))
    (Utilities|Casting|CastToBP_FirstPersonCharacter OtherActor)
    (Audio|Components|Audio|FadeOut (Variables|Default|GetSpeakerVoice) 5.0 0.0 "Linear" :!class /Script/Engine.AudioComponent)
    (Utilities|FlowControl|Delay 5.0)
    (Audio|Components|Audio|Stop (Variables|Default|GetSpeakerVoice))
    (Variables|Default|SetIsActivated false)))

(event EventBeginPlay
  (Variables|Default|SetIsActivated false))

(event Collision|EventActorBeginOverlap
  (params (OtherActor :type Actor%20Object%20Reference)))

(event EventTick
  (params (DeltaSeconds :type Float%20%28single-precision%29)))

(fn ConstructionScript)